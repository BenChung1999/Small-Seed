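; BP_Branch is a branch object that can be placed and attached to whatever component a hit result reports.
; Place applies the tree material to the mesh, enables collision on the capsule and box, and turns on gravity and physics simulation for the capsule.
; It then binds the capsule to the hit component through two physics constraints, so the branch hangs as a simulated body.
; The event graph and construction script are empty.
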(event `self.ReceiveActorBeginOverlap`
  (params (OtherActor :type "Actor Object Reference")))

(event `self.ReceiveTick`
  (params (DeltaSeconds :type "Float (single-precision)")))

(fn `Place`
  (params (`Hit Result` :type "HitResult Structure"))
  (bind (_bblockinghit _binitialoverlap _time _distance _location _impactpoint _normal _impactnormal _physmat _hitactor _hitcomponent) (`GameplayStatics.BreakHitResult` `Hit Result`))
  (bind _capsule (`self.Capsule`))
  (bind _capsule_2 (`self.Capsule`))
  (`|ExecutionSequence`
    (:`then_0`
      ;[1 1 1] Init Branch Setting
      (`PrimitiveComponent.SetMaterial` (`self.BranchMesh`) 0 "/Game/Materials/M_Tree_One.M_Tree_One")
      (`PrimitiveComponent.SetCollisionEnabled` _capsule "QueryAndPhysics")
      (`PrimitiveComponent.SetCollisionEnabled` (`self.Box`) "QueryAndPhysics")
      (`PrimitiveComponent.SetEnableGravity` _capsule true)
      (`PrimitiveComponent.SetSimulatePhysics` _capsule true))
    (:`then_1`
      (`PhysicsConstraintComponent.SetConstrainedComponents` (`self.PhysicsConstraint`) _capsule_2 "None" _hitcomponent "None")
      (`PhysicsConstraintComponent.SetConstrainedComponents` (`self.PhysicsConstraint1`) _capsule_2 "None" _hitcomponent "None"))))

(fn `UserConstructionScript`)