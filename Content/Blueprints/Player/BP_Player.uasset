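; Player pawn that walks with FloatingPawnMovement, climbs magical trees and branches, and places branches in the world.
; A per-tick camera line trace supplies the hit used for climbing, placement and right-click removal.
; Climbing disables gravity and drains timer-driven stamina, which recovers otherwise and shows a main UI widget at start.
; Holding left click previews a branch aligned to the surface normal, the wheel scales it, and release places it with Niagara effects.
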(event `self.ReceiveBeginPlay`
  (`KismetSystemLibrary.K2_SetTimerDelegate` (delegate `StaminaManage`) 1.0 true)
  (bind _returnvalue (`|CreateWidget` "/Game/UI/WBP_MainUI.WBP_MainUI_C"))
  (`UserWidget.AddToViewport` _returnvalue 0))

(event `StaminaManage`
  (if (`self.IsClimbing`)
    (set `self.Stamina` (`KismetMathLibrary.FMax` (- (`self.Stamina`) (`self.StaminaChangeRate`))))
    (else
      (set `self.Stamina` (`KismetMathLibrary.FMin` (+ (`self.Stamina`) (`self.StaminaChangeRate`)) 100.0)))))

(event `self.ReceiveTick`
  (params (DeltaSeconds :type "Float (single-precision)"))
  (bind _returnvalue (`GameplayStatics.GetPlayerCameraManager` 0))
  (bind _returnvalue_2 (`self.GetActorForwardVector` _returnvalue))
  (bind _returnvalue_3 (`self.K2_GetActorLocation` _returnvalue))
  ;[1 1 1] Can not Branch
  (bind _outhit (`KismetSystemLibrary.LineTraceSingleForObjects` :`Start` (+ _returnvalue_3 _returnvalue_2) :`End` (+ _returnvalue_3 (* _returnvalue_2 (`self.ArmLength`))) :`ObjectTypes` (`self.Object Types`) :`bTraceComplex` true :`DrawDebugType` "ForOneFrame"))
  (set `self.HittingResult` _outhit))

(event `InputAxis|MouseVertical`
  (params (AxisValue :type "Float (single-precision)"))
  ;[1 1 1] Mouse Move
  (`self.AddControllerPitchInput` AxisValue))

(event `InputAxis|MouseHorizontal`
  (params (AxisValue :type "Float (single-precision)"))
  ;[1 1 1] Mouse Move
  (`self.AddControllerYawInput` AxisValue))

(event `InputAxis|MoveVertical`
  (params (AxisValue :type "Float (single-precision)"))
  (bind (_returnvalue_x _returnvalue_y) (`KismetMathLibrary.BreakVector` (* (`self.GetActorForwardVector` (`GameplayStatics.GetPlayerCameraManager` 0)) (* AxisValue (`self.VeritcalSpeed`)))))
  ;[1 1 1] WASD
  (if (and (`self.IsClimbing`) (< AxisValue 0.0))
    (set `self.VeritcalSpeed` 0.0)
    (else
      (set `self.VeritcalSpeed` 0.8)))
  (`PawnMovementComponent.AddInputVector` (`self.FloatingPawnMovement`) (`KismetMathLibrary.MakeVector` _returnvalue_x _returnvalue_y) false))

(event `InputAxis|MoveHorizontal`
  (params (AxisValue :type "Float (single-precision)"))
  ;[1 1 1] WASD
  (if (`self.IsClimbing`)
    (set `self.HorizontalSpeed` 0.2)
    (else
      (set `self.HorizontalSpeed` 0.5)))
  (`PawnMovementComponent.AddInputVector` (`self.FloatingPawnMovement`) (* (`self.GetActorRightVector` (`GameplayStatics.GetPlayerCameraManager` 0)) (* AxisValue (`self.HorizontalSpeed`))) false))

(event `InputAxis|MoveUp`
  (params (AxisValue :type "Float (single-precision)"))
  (bind (_bblockinghit _binitialoverlap _time _distance _location _impactpoint _normal _impactnormal _physmat _hitactor) (`GameplayStatics.BreakHitResult` (`self.HittingResult`)))
  ;[1 1 1] WASD
  (if (or (`.bSuccess` (cast `/Game/Blueprints/Objects/BP_SmallMagicalTree` _hitactor :!pure true)) (`.bSuccess` (cast `/Game/Blueprints/Objects/BP_Branch` _hitactor :!pure true)))
    (if (> (`self.Stamina`) 0.0)
      (if (and (> AxisValue 0.0) (< (`KismetMathLibrary.Vector_Distance` _impactpoint (`self.K2_GetActorLocation`)) 200.0))
        (`PrimitiveComponent.SetEnableGravity` (`self.Box`) false)
        (`PawnMovementComponent.AddInputVector` (`self.FloatingPawnMovement`) (* (`self.GetActorUpVector` (`GameplayStatics.GetPlayerCameraManager` 0)) (* AxisValue (`self.UpSpeed`))) false)
        (set `self.IsClimbing` true))
      (else
        (`PrimitiveComponent.SetEnableGravity` (`self.Box`) true :!label _label)
        (set `self.IsClimbing` false)))
    (else
      (goto _label))))

(event `InputAxisKey|MouseWheelAxis`
  (params (AxisValue :type "Float (single-precision)"))
  (bind _scalelimited (`self.ScaleLimited`))
  (bind (_bblockinghit _binitialoverlap _time _distance _location _impactpoint _normal _impactnormal _physmat _hitactor) (`GameplayStatics.BreakHitResult` (`self.HittingResult`)))
  (bind _returnvalue (* AxisValue (`self.ScaleSpeed`)))
  (bind (_returnvalue_x _returnvalue_y _returnvalue_z) (`KismetMathLibrary.BreakVector` (`self.GetActorScale3D` _hitactor)))
  ;[1 1 1] Mosue Input
  (bind _currentbranch (`self.CurrentBranch`)
    (:`then`
      (cast `/Game/Blueprints/Objects/BP_Branch` _hitactor
        (:`then`
          (bind (_returnvalue_x_2 _returnvalue_y_2 _returnvalue_z_2) (`KismetMathLibrary.BreakVector` (`self.GetActorScale3D` _currentbranch)))
          (bind _returnvalue_2 (+ _returnvalue_x_2 _returnvalue))
          (bind _returnvalue_3 (+ _returnvalue_y_2 _returnvalue))
          (bind _returnvalue_4 (+ _returnvalue_z_2 _returnvalue))
          (`self.SetActorScale3D` _currentbranch (`KismetMathLibrary.MakeVector` (`KismetMathLibrary.FMin` (* _returnvalue_x _scalelimited) _returnvalue_2) (`KismetMathLibrary.FMin` (* _returnvalue_y _scalelimited) _returnvalue_3) (`KismetMathLibrary.FMin` (* _returnvalue_z _scalelimited) _returnvalue_4))))
        (:`CastFailed`
          (`self.SetActorScale3D` _currentbranch (`KismetMathLibrary.MakeVector` _returnvalue_2 _returnvalue_3 _returnvalue_4)))))
    (:`else`)))

(event `Key|LeftMouseButton`
  (params (Key :type "Key Structure"))
  (bind _hittingresult (`self.HittingResult`))
  (bind _niagara (`self.Niagara`))
  ;[1 1 1] Mosue Input
  (:`Pressed`
    (bind _returnvalue (`|SpawnActorFromClass` "/Game/Blueprints/Objects/BP_Branch.BP_Branch_C" (`KismetMathLibrary.MakeTransform` (0.0 0.0 0.0)) "AdjustIfPossibleButAlwaysSpawn" "MultiplyWithRoot" null null))
    (bind _output_get (set `self.CurrentBranch` _returnvalue))
    (`PrimitiveComponent.SetMaterial` (`/Game/Blueprints/Objects/BP_Branch.BranchMesh` _output_get) 0 "/Game/Materials/M_Preview.M_Preview")
    (bind _returnvalue_2 (`KismetSystemLibrary.K2_SetTimerDelegate` (`|CreateDelegate` :!event `SpawnTree`) 0.05 true))
    (set `self.TreePreviewTimer` _returnvalue_2))
  (:`Released`
    (`KismetSystemLibrary.K2_ClearAndInvalidateTimerHandle` (`self.TreePreviewTimer`))
    (`/Game/Blueprints/Objects/BP_Branch.Place` (`self.CurrentBranch`) _hittingresult)
    (`SceneComponent.K2_SetWorldLocation` _niagara (`.ImpactPoint` (`GameplayStatics.BreakHitResult` _hittingresult)) false true)
    (`ActorComponent.Activate` _niagara true)
    (set `self.CurrentBranch` null)))

(event `Key|RightMouseButton`
  (params (Key :type "Key Structure"))
  ;[1 1 1] Mosue Input
  (:`Pressed`
    (bind _asbp_branch (cast `/Game/Blueprints/Objects/BP_Branch` (`.HitActor` (`GameplayStatics.BreakHitResult` (`self.HittingResult`)))))
    (`self.K2_DestroyActor` _asbp_branch)
    (set `self.CurrentBranch` null)
    (`KismetSystemLibrary.K2_ClearAndInvalidateTimerHandle` (`self.TreePreviewTimer`))))

(event `SpawnTree`
  (bind (_bblockinghit _binitialoverlap _time _distance _location _impactpoint _normal _impactnormal) (`GameplayStatics.BreakHitResult` (`self.HittingResult`)))
  (`self.K2_SetActorLocationAndRotation` (`self.CurrentBranch`) _impactpoint (`KismetMathLibrary.Conv_VectorToRotator` _impactnormal) false false))

(fn `UserConstructionScript`)